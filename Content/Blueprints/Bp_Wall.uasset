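; Bp_Wall is a temporary wall actor that rises when spawned, stays for a set lifetime, then retracts and destroys itself.
; BeginPlay plays the RiseMovement timeline, waits out its length plus TimeToLive, reverses it, then destroys the actor after the same length.
; The timeline update lerps the Cube's world location between the Start and End components without sweeping.
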(event EventBeginPlay
  (bind _risemovement (Variables|Default|GetRiseMovement))
  (bind _risemovement_2 (Variables|Default|GetRiseMovement))
  (Components|Timeline|PlayfromStart _risemovement_2)
  (Utilities|FlowControl|Delay (Components|Timeline|GetTimelineLength _risemovement_2))
  (Utilities|FlowControl|Delay (Variables|Default|GetTimeToLive))
  (Components|Timeline|ReversefromEnd _risemovement)
  (Utilities|FlowControl|Delay (Components|Timeline|GetTimelineLength _risemovement))
  (Actor|DestroyActor))

(event Collision|EventActorBeginOverlap
  (params (OtherActor :type Actor%20Object%20Reference)))

(event EventTick
  (params (DeltaSeconds :type Float%20%28single-precision%29)))

(fn ConstructionScript)