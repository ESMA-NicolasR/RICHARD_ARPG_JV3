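; Shopkeeper NPC Blueprint that sells spells to the player through a shop widget.
; On BeginPlay it creates a WBP_Shop widget and fills one slot per entry in SpellsToSell, passing itself as the shopkeeper.
; It extends its parent's dialogue events to show the shop when dialogue starts and remove it when it ends.
; SellItem forwards the chosen slot to the widget.
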(event EventBeginPlay
  (|CallParentFunction)
  (CallFunction|InitShop))

(event Collision|EventActorBeginOverlap
  (params (OtherActor :type Actor%20Object%20Reference))
  (|CallParentFunction OtherActor) ; This node is disabled and will not be called.\nDrag off pins to build functionality.
)

(event EventTick
  (params (DeltaSeconds :type Float%20%28single-precision%29))
  (|CallParentFunction DeltaSeconds) ; This node is disabled and will not be called.\nDrag off pins to build functionality.
)

(event EventStartDialogue
  (|CallParentFunction)
  (UserInterface|Viewport|AddtoViewport (Variables|Default|GetShopUI) 0))

(event EventEndDialogue
  (|CallParentFunction)
  (Widget|RemovefromParent (Variables|Default|GetShopUI)))

(fn ConstructionScript
  (|CallParentFunction))

(fn SellItem
  (params (Slot :type Integer))
  (Default|SellItem (Variables|Default|GetShopUI) Slot))

(fn InitShop
  (bind _returnvalue (UserInterface|CreateWidget "/Game/UI/WBP_Shop.WBP_Shop_C"))
  (Variables|Default|SetShopUI _returnvalue)
  (for (_array_element _array_index) (Variables|Default|GetSpellsToSell)
    (Default|InitItem (Variables|Default|GetShopUI) _array_index _array_element self)))