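; BP_DA_Spell is a spell Blueprint, apparently a data asset, that carries a name and resource cost and handles the attempt to cast it.
; LaunchSpell asks the passed-in Controller to spend the cost as mana through TrySpendMana.
; It only prints a success or failure message with the spell's name, with no spell effect in this graph.
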(fn LaunchSpell
  (params (Controller :type BP%20Top%20Down%20Controller%20Object%20Reference))
  (bind _canspend (Default|TrySpendMana Controller (Variables|Default|GetResourceCost)))
  (if _canspend
    (Development|PrintString 0 (Utilities|String|Append "Casting spell : " (Utilities|String|ToString(Name) (Variables|Default|GetName))))
    (else
      (Development|PrintString 0 (Utilities|String|Append "Could not cast spell :" (Utilities|String|ToString(Name) (Variables|Default|GetName)))))))