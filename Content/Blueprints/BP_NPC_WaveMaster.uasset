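; BP_NPC_WaveMaster is a dialogue NPC that lets the player launch and track enemy waves.
; Its world-space button widget, shown during dialogue only while no wave runs, holds a reference to it.
; StartWave closes the dialogue, triggers every BP_EnemySpawner and sums their planned spawns.
; The player controller's enemy-killed event decrements that count, updates the enemy UI and clears the wave flag at zero.
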(event Custom|OnEnemyKilled_Event
  (bind _result (Math|Integer|DecrementInt (Variables|Default|GetEnemiesRemaining))
    (:%20%20
      (CallFunction|UpdateEnemiesUI)
      (Variables|Default|SetWaveIsOnGoing (> _result 0)))))

(event EventBeginPlay
  (|CallParentFunction)
  (CallFunction|ChangeDialogue "Salutation aventurier, êtes-vous prêt à passer un coup de brosse sur des ennemis ?")
  (bind _aswbp_wave_button (Utilities|Casting|CastToWBP_WaveButton (UserInterface|GetWidget (Variables|Default|GetWaveButtonWidget))))
  (Variables|/Game/UI/WBP_WaveButton.WBP_WaveButton_C|SetWaveMaster _aswbp_wave_button self)
  (EventDispatchers|AssignOnEnemyKilled (CallFunction|GetPlayerController) (delegate Custom|OnEnemyKilled_Event)))

(event Collision|EventActorBeginOverlap
  (params (OtherActor :type Actor%20Object%20Reference))
  (|CallParentFunction OtherActor) ; This node is disabled and will not be called.\nDrag off pins to build functionality.
)

(event EventTick
  (params (DeltaSeconds :type Float%20%28single-precision%29))
  (|CallParentFunction DeltaSeconds) ; This node is disabled and will not be called.\nDrag off pins to build functionality.
)

(event EventStartDialogue
  (|CallParentFunction)
  (Rendering|SetVisibility (Variables|Default|GetWaveButtonWidget) (not (Variables|Default|GetWaveIsOnGoing)) false)
  (Rendering|SetVisibility (Variables|Default|GetQuitButtonWidget) true false))

(event EventEndDialogue
  (|CallParentFunction)
  (Rendering|SetVisibility (Variables|Default|GetWaveButtonWidget) false false)
  (Rendering|SetVisibility (Variables|Default|GetQuitButtonWidget) false false))

(fn ConstructionScript
  (|CallParentFunction))

(fn StartWave
  (if (not (Variables|Default|GetWaveIsOnGoing))
    (Variables|Default|SetWaveIsOnGoing true)
    (CallFunction|EndDialogue)
    (bind _outactors (Actor|GetAllActorsOfClass "/Game/Blueprints/BP_EnemySpawner.BP_EnemySpawner_C"))
    (for _array_element _outactors
      (Default|StartWave _array_element)
      (Variables|Default|SetEnemiesRemaining (+ (* (Variables|/Game/Blueprints/BP_EnemySpawner.BP_EnemySpawner_C|GetSpawnNb _array_element) (Variables|/Game/Blueprints/BP_EnemySpawner.BP_EnemySpawner_C|GetSpawnPerTick _array_element)) (Variables|Default|GetEnemiesRemaining))))
    (CallFunction|UpdateEnemiesUI)))

(fn UpdateEnemiesUI
  (Default|UpdateEnemiesUI (CallFunction|GetPlayerController) (Variables|Default|GetEnemiesRemaining)))