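; Enemy spawner actor that releases a wave of EnemyClass actors at its SpawnPoint transform, optionally starting on BeginPlay through StartOnSpawn.
; StartWave enables Tick, sets its interval to SpawnCooldown and loads RemainingToSpawn from SpawnNb.
; Tick doubles as the spawn timer: each step decrements the counter and spawns a batch sized by SpawnPerTick, so SpawnNb counts batches.
; Tick disables itself once the counter runs out.
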(event EventBeginPlay
  (if (Variables|Default|GetStartOnSpawn)
    (CallFunction|StartWave)))

(event Collision|EventActorBeginOverlap
  (params (OtherActor :type Actor%20Object%20Reference)))

(event EventTick
  (params (DeltaSeconds :type Float%20%28single-precision%29))
  (if (> (Variables|Default|GetRemainingToSpawn) 0)
    (Math|Integer|DecrementInt (Variables|Default|GetRemainingToSpawn)
      (:%20%20
        (for _index (range 0 (Variables|Default|GetSpawnPerTick))
          (Game|SpawnActorfromClass (Variables|Default|GetEnemyClass) (Transformation|GetWorldTransform (Variables|Default|GetSpawnPoint)) "Undefined" "MultiplyWithRoot" 0 0))))
    (else
      (Actor|Tick|SetActorTickEnabled false))))

(fn ConstructionScript)

(fn StartWave
  (Actor|Tick|SetActorTickEnabled true)
  (Actor|Tick|SetActorTickInterval (Variables|Default|GetSpawnCooldown))
  (Variables|Default|SetRemainingToSpawn (Variables|Default|GetSpawnNb)))